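; King of the Hill game mode that decides where MSPs and FOBs may be placed.
; It stores the registered ruleset and reads its lattice and current flag for the checks.
; MSP placement fails inside the sphere of any main base or the current flag, using squared-distance tests.
; FOB placement defers to the lattice and reports an exclusion-zone reason on failure; both checks ignore team.
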(event Custom|OnRulesetRegistered
  (params (Ruleset :type BP%20Ruleset%20KOTH%20Object%20Reference))
  (Utilities|IsValid Ruleset
    (:Is%20Valid
      (Variables|Default|SetRuleset Ruleset))))

(event EventBeginPlay
  (|CallParentFunction) ; This node is disabled and will not be called.\nDrag off pins to build functionality.
)

(event EventTick
  (params (DeltaSeconds :type Float%20%28single-precision%29))
  (|CallParentFunction DeltaSeconds) ; This node is disabled and will not be called.\nDrag off pins to build functionality.
)

(fn ConstructionScript
  (|CallParentFunction))

(fn IsMSPPlacementValid
  (params (Location :type Vector :default "0, 0, 0") (Team :type ESQTeam%20Enum :default "Team_Neutral"))
  (bind _ruleset (Variables|Default|GetRuleset))
  (bind _currentflag (Variables|/KOTH/GameMode/BP_Ruleset_KOTH.BP_Ruleset_KOTH_C|GetCurrentFlag _ruleset))
  (bind _output_get (LocalVariables|SetForbiddenLocations (Variables|/KOTH/GameMode/BP_PS_KOTH_Lattice.BP_PS_KOTH_Lattice_C|GetMainBases (Variables|/KOTH/GameMode/BP_Ruleset_KOTH.BP_Ruleset_KOTH_C|GetLattice _ruleset))))
  (Utilities|IsValid _currentflag
    (:Is%20Valid
      (Utilities|Array|Add _output_get _currentflag))
    (:Is%20Not%20Valid
      _))
  (for _array_element (LocalVariables|GetForbiddenLocations)
    (if (> (Math|Float|Square (Components|Sphere|GetScaledSphereRadius (Variables|/Game/Blueprints/Placeable/CaptureZones/BP_PSCaptureZoneNew.BP_PSCaptureZoneNew_C|GetSphere _array_element))) (Math|Vector|VectorLengthSquared (- Location (Transformation|GetActorLocation _array_element))))
      (return false)))
  (return true))

(fn IsFOBPlacementValid
  (params (Location :type Vector :default "0, 0, 0") (Team :type ESQTeam%20Enum :default "Team_Neutral"))
  (bind _valid (Default|IsFOBPlacementValid (Variables|/KOTH/GameMode/BP_Ruleset_KOTH.BP_Ruleset_KOTH_C|GetLattice (Variables|Default|GetRuleset)) Location))
  (return _valid (select _valid "VALID" "EXCLUSION_ZONE")))