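; King of the Hill HUD that shows capture zone visibility, objective countdowns and the break between objectives.
; On BeginPlay it caches the zones, KOTH lattice and staging actor, hides non-main zone icons and starts a one-second timer writing remaining time into the current flag's objective texts.
; Tick syncs icons to team visibility, toggles the capture widget by pawn distance and, outside staging, shows the next-objective countdown in the staging timer widget.
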(event Custom|ShowFlag
  (bind _asbp_ps_game_mode_koth (Utilities|Casting|CastToBP_PS_GameMode_KOTH (Game|GetGameMode)))
  (Utilities|IsValid (Variables|/KOTH/GameMode/BP_Ruleset_KOTH.BP_Ruleset_KOTH_C|GetCurrentFlag (Variables|/KOTH/GameMode/BP_PS_GameMode_KOTH.BP_PS_GameMode_KOTH_C|GetRuleset _asbp_ps_game_mode_koth))
    (:Is%20Valid
      (Variables|/Script/Squad.SQMapItemComponent|SetbIsVisible (Variables|/Game/Blueprints/Placeable/CaptureZones/BP_PSCaptureZoneNew.BP_PSCaptureZoneNew_C|GetSQMapIcon (Variables|/KOTH/GameMode/BP_Ruleset_KOTH.BP_Ruleset_KOTH_C|GetCurrentFlag (Variables|/KOTH/GameMode/BP_PS_GameMode_KOTH.BP_PS_GameMode_KOTH_C|GetRuleset _asbp_ps_game_mode_koth))) true))))

(event Custom|TimeRemainingMarkerUpdate
  (bind _lattice (Variables|Default|GetLattice))
  (bind _currentflag (Variables|/KOTH/GameMode/BP_PS_KOTH_Lattice.BP_PS_KOTH_Lattice_C|GetCurrentFlag _lattice))
  (Utilities|IsValid _lattice
    (:Is%20Valid
      (Utilities|IsValid _currentflag
        (:Is%20Valid
          (CallFunction|UpdateFlagTimer _currentflag))))))

(event EventBeginPlay
  (|CallParentFunction)
  (Utilities|FlowControl|Sequence
    (:then_0
      (bind _outactors (Actor|GetAllActorsOfClass "/Game/Blueprints/Placeable/CaptureZones/BP_PSCaptureZoneNew.BP_PSCaptureZoneNew_C"))
      (bind _output_get (Variables|Default|SetAllFlags _outactors))
      (for _array_element _output_get
        (if (not (Variables|/Game/Blueprints/Placeable/CaptureZones/BP_PSCaptureZoneNew.BP_PSCaptureZoneNew_C|GetbIsMain _array_element))
          (Variables|/Script/Squad.SQMapItemComponent|SetbIsVisible (Variables|/Game/Blueprints/Placeable/CaptureZones/BP_PSCaptureZoneNew.BP_PSCaptureZoneNew_C|GetSQMapIcon _array_element) false)))
      (bind _outactors_2 (Actor|GetAllActorsOfClass "/KOTH/GameMode/BP_PS_KOTH_Lattice.BP_PS_KOTH_Lattice_C"))
      (Utilities|IsValid (Utilities|Array|Get(acopy) _outactors_2)
        (:Is%20Valid
          (Variables|Default|SetLattice (Utilities|Array|Get(acopy) _outactors_2))
          (Utilities|Time|SetTimerbyEvent (delegate Custom|TimeRemainingMarkerUpdate) 1.0 true))))
    (:then_1
      (bind _outactors_3 (Actor|GetAllActorsOfClass "/Game/Gameplay/GameplayBorder/Gameplay_TeamPrep.Gameplay_TeamPrep_C"))
      (Variables|Default|SetStaging (Utilities|Array|Get(acopy) _outactors_3)))))

(event Collision|EventActorBeginOverlap
  (params (OtherActor :type Actor%20Object%20Reference))
  (|CallParentFunction OtherActor) ; This node is disabled and will not be called.\nDrag off pins to build functionality.
)

(event EventTick
  (params (DeltaSeconds :type Float%20%28single-precision%29))
  (|CallParentFunction DeltaSeconds)
  (CallFunction|UpdateFlagVisibility)
  (CallFunction|UpdateBreakTimer))

(fn ConstructionScript
  (|CallParentFunction))

(fn UpdateFlagVisibility
  (for _array_element (Variables|Default|GetAllFlags)
    (Variables|/Script/Squad.SQMapItemComponent|SetbIsVisible (Variables|/Game/Blueprints/Placeable/CaptureZones/BP_PSCaptureZoneNew.BP_PSCaptureZoneNew_C|GetSQMapIcon _array_element) (Utilities|Array|Get(acopy) (Variables|/Game/PostScriptum/Blueprints/BP_PSCaptureZoneComponent.BP_PSCaptureZoneComponent_C|GetbVisibleForTeam (Variables|/Game/Blueprints/Placeable/CaptureZones/BP_CaptureZone.BP_CaptureZone_C|GetBP_PSCaptureZoneComponent _array_element))))
    (bind _isincap (CallFunction|IsPlayerinCap _array_element))
    (if (and (Utilities|Array|Get(acopy) (Variables|/Game/PostScriptum/Blueprints/BP_PSCaptureZoneComponent.BP_PSCaptureZoneComponent_C|GetbVisibleForTeam (Variables|/Game/Blueprints/Placeable/CaptureZones/BP_CaptureZone.BP_CaptureZone_C|GetBP_PSCaptureZoneComponent _array_element))) _isincap)
      (LocalVariables|SetIsPlayerInVisibleCap true)))
  (CallFunction|SetTacticalHudMarkerVisibility (LocalVariables|GetIsPlayerInVisibleCap)))

(fn IsPlayerinCap
  (params (Flag :type BP%20PS%20Capture%20Zone%20New%20Object%20Reference))
  (bind _self self)
  (bind _returnvalue (Class|HUD|GetOwningPawn _self))
  (Utilities|IsValid _returnvalue
    (:Is%20Valid
      (Utilities|IsValid Flag
        (:Is%20Valid
          (return (> (Math|Float|Square (Components|Sphere|GetScaledSphereRadius (Variables|/Game/Blueprints/Placeable/CaptureZones/BP_PSCaptureZoneNew.BP_PSCaptureZoneNew_C|GetSphere Flag))) (Math|Vector|VectorLengthSquared (- (Transformation|GetActorLocation Flag) (Transformation|GetActorLocation _returnvalue))))))))
    (:Is%20Not%20Valid
      (return false))))

(fn SetTacticalHudMarkerVisibility
  (params (Is%20Visible :type Boolean))
  (bind _basehudwidget (Variables|Default|GetBaseHudWidget))
  (Utilities|IsValid _basehudwidget
    (:Is%20Valid
      (bind _asumg_ps_base_hud (Utilities|Casting|CastToUMG_PS_BaseHUD _basehudwidget))
      (if Is%20Visible
        (Widget|SetVisibility (Variables|/Game/PostScriptum/UI/Widgets/BP_PS_CaptureZoneStatusWidget.BP_PS_CaptureZoneStatusWidget_C|GetCanvasPanel_566 (Variables|/Game/PostScriptum/UI/UMG_PS_BaseHUD.UMG_PS_BaseHUD_C|GetBP_PS_CaptureZoneStatusWidget_43 _asumg_ps_base_hud)) "Visible")
        (else
          (Widget|SetVisibility (Variables|/Game/PostScriptum/UI/Widgets/BP_PS_CaptureZoneStatusWidget.BP_PS_CaptureZoneStatusWidget_C|GetCanvasPanel_566 (Variables|/Game/PostScriptum/UI/UMG_PS_BaseHUD.UMG_PS_BaseHUD_C|GetBP_PS_CaptureZoneStatusWidget_43 _asumg_ps_base_hud)) "Hidden"))))))

(fn UpdateFlagTimer
  (params (Flag :type BP%20PS%20Capture%20Zone%20New%20Object%20Reference))
  (bind _lattice (Variables|Default|GetLattice))
  (bind _activeflagremainingtime (Variables|/KOTH/GameMode/BP_PS_KOTH_Lattice.BP_PS_KOTH_Lattice_C|GetActiveFlagRemainingTime _lattice))
  (bind (_remainder _returnvalue) (Math|Float|Division(WholeandRemainder) _activeflagremainingtime 6e+01))
  (bind _returnvalue_2 (Utilities|Text|ToText(Integer) _returnvalue false true 2 2))
  (bind _returnvalue_3 (Utilities|Text|ToText(Float) _remainder "HalfToEven" false true 2 2 0 0))
  (bind _returnvalue_4 (Utilities|String|ToString(Text) _returnvalue_3))
  (bind _returnvalue_5 (Utilities|String|ToString(Text) _returnvalue_2))
  (bind _returnvalue_6 (Utilities|String|Append _returnvalue_5 ":" _returnvalue_4))
  (bind _returnvalue_7 (Utilities|Text|ToText(String) _returnvalue_6))
  (Variables|/Game/Blueprints/Placeable/CaptureZones/BP_PSCaptureZoneNew.BP_PSCaptureZoneNew_C|SetAttackerObjectiveText Flag _returnvalue_7)
  (Variables|/Game/Blueprints/Placeable/CaptureZones/BP_PSCaptureZoneNew.BP_PSCaptureZoneNew_C|SetDefenderObjectiveText Flag _returnvalue_7))

(fn UpdateBreakTimer
  (bind _basehudwidget (Variables|Default|GetBaseHudWidget))
  (bind _lattice (Variables|Default|GetLattice))
  (bind _breakremainingtime (Variables|/KOTH/GameMode/BP_PS_KOTH_Lattice.BP_PS_KOTH_Lattice_C|GetBreakRemainingTime _lattice))
  (bind (_remainder _returnvalue) (Math|Float|Division(WholeandRemainder) _breakremainingtime 6e+01))
  (Utilities|IsValid _basehudwidget
    (:Is%20Valid
      (bind _asumg_ps_base_hud (Utilities|Casting|CastToUMG_PS_BaseHUD _basehudwidget))
      (bind _isstagingphase (CallFunction|IsStagingPhase))
      (if (not _isstagingphase)
        (if (> _breakremainingtime 0.0)
          (Widget|SetVisibility (Variables|/Game/PostScriptum/UI/UMG_PS_BaseHUD.UMG_PS_BaseHUD_C|GetUMG_StagingTimerText _asumg_ps_base_hud) "Visible")
          (Rendering|Components|TextRender|SetText (Variables|/Script/Squad.SQStagingTimerText|GetTextBlockCPP (Variables|/Game/PostScriptum/UI/UMG_PS_BaseHUD.UMG_PS_BaseHUD_C|GetUMG_StagingTimerText _asumg_ps_base_hud)) (Utilities|Text|ToText(String) (Utilities|String|Append "New objective spawning in " (Utilities|String|ToString(Text) (Utilities|Text|ToText(Integer) _returnvalue false true 2 2)) ":" (Utilities|String|ToString(Text) (Utilities|Text|ToText(Float) _remainder "HalfToEven" false true 2 2 0 0)))))
          (Appearance|SetColorandOpacity (Variables|/Game/UI/Widgets/HUD/StateIndicators/UMG_StagingTimerText.UMG_StagingTimerText_C|GetBlackBG (Variables|/Game/PostScriptum/UI/UMG_PS_BaseHUD.UMG_PS_BaseHUD_C|GetUMG_StagingTimerText _asumg_ps_base_hud)) (Utilities|Struct|MakeLinearColor 0.0 0.0 0.0 0.5) :!class /Script/UMG.Image)
          (Class|CanvasPanelSlot|SetPosition (Class|WidgetLayoutLibrary|SlotasCanvasSlot (Variables|/Game/PostScriptum/UI/UMG_PS_BaseHUD.UMG_PS_BaseHUD_C|GetUMG_StagingTimerText _asumg_ps_base_hud)) "(X=63.326000,Y=-53.660000)")
          (elif (Widget|IsVisible (Variables|/Game/PostScriptum/UI/UMG_PS_BaseHUD.UMG_PS_BaseHUD_C|GetUMG_StagingTimerText _asumg_ps_base_hud))
            (Widget|SetVisibility (Variables|/Game/PostScriptum/UI/UMG_PS_BaseHUD.UMG_PS_BaseHUD_C|GetUMG_StagingTimerText _asumg_ps_base_hud) "Hidden")))))))

(fn IsStagingPhase
  (return (Utilities|IsValid (Variables|Default|GetStaging))))