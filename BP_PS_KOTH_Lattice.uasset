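; King-of-the-hill lattice actor that paints a FOB overlay for the map, marking forbidden zones around main bases and the current flag.
; It redraws on lattice updates on the server and on a looping timer where cosmetics run.
; Zone spheres are converted to texture space using the world settings' map corners.
; Each is stamped as a circle into a cleared render target through a dynamic brush material.
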(event Custom|LatticeUpdated
  (CallFunction|UpdateFobOverlay))

(event EventBeginPlay
  (Networking|SwitchHasAuthority
    (:Authority
      (EventDispatchers|BindEventtoOnLatticeUpdated (delegate Custom|LatticeUpdated))
      (CallFunction|LatticeUpdated))
    (:Remote
      _))
  (Networking|CanExecuteCosmeticEvents
    (:True
      (bind _returnvalue (Rendering|Material|CreateDynamicMaterialInstance "/Game/PostScriptum/UI/Materials/M_MSPHeatMapDrawer_Inst.M_MSPHeatMapDrawer_Inst" "None" :!class /Script/Engine.KismetMaterialLibrary))
      (Variables|Default|SetOverlayBrushMaterial _returnvalue)
      (Utilities|Time|SetTimerbyEvent (delegate Custom|LatticeUpdated) 1.0 true))))

(event Collision|EventActorBeginOverlap
  (params (OtherActor :type Actor%20Object%20Reference)))

(event EventTick
  (params (DeltaSeconds :type Float%20%28single-precision%29)))

(fn ConstructionScript)

(fn UpdateFobOverlay
  (bind _overlaybrushmaterial (Variables|Default|GetOverlayBrushMaterial))
  (Rendering|ClearRenderTarget2D self (Variables|Default|GetOverlayRenderToTexture))
  (Utilities|IsValid (Variables|Default|GetOverlayBrushMaterial)
    (:Is%20Valid
      (bind _instructions (CallFunction|GetFOBOverlayDrawingInstructions))
      (for _array_element _instructions
        (Rendering|Material|SetTextureParameterValue _overlaybrushmaterial "Stencil" "/Game/PostScriptum/UI/Textures/T_Circle.T_Circle")
        (Rendering|Material|SetScalarParameterValue _overlaybrushmaterial "Diameter" (.Diameter (Utilities|Struct|BreakMSPOverlayDrawingInstruction _array_element)) :!class /Script/Engine.MaterialInstanceDynamic)
        (Rendering|Material|SetVectorParameterValue _overlaybrushmaterial "Position" (.Location (Utilities|Struct|BreakMSPOverlayDrawingInstruction _array_element)) :!class /Script/Engine.MaterialInstanceDynamic)
        (Rendering|DrawMaterialtoRenderTarget self (Variables|Default|GetOverlayRenderToTexture) (Variables|Default|GetOverlayBrushMaterial))))))

(fn GetFOBOverlayDrawingInstructions
  (bind _currentflag (Variables|Default|GetCurrentFlag))
  (bind _returnvalue (Class|SQBlueprintLibrary|GetWorldSettings))
  (bind _assqworld_settings (Utilities|Casting|CastToSQWorldSettings _returnvalue))
  (LocalVariables|SetCornerZeroLoc (Transformation|GetActorLocation (Variables|/Script/Squad.SQWorldSettings|GetMapTextureCornerZero _assqworld_settings)))
  (LocalVariables|SetCornerOneLoc (Transformation|GetActorLocation (Variables|/Script/Squad.SQWorldSettings|GetMapTextureCornerOne _assqworld_settings)))
  (LocalVariables|SetWorldScale (/ 1.0 (Math|Float|Max(Float) (Math|Float|Absolute(Float) (- (.X (Math|Vector|BreakVector (Transformation|GetActorLocation (Variables|/Script/Squad.SQWorldSettings|GetMapTextureCornerZero _assqworld_settings)))) (.X (Math|Vector|BreakVector (Transformation|GetActorLocation (Variables|/Script/Squad.SQWorldSettings|GetMapTextureCornerOne _assqworld_settings)))))) (Math|Float|Absolute(Float) (- (.Y (Math|Vector|BreakVector (Transformation|GetActorLocation (Variables|/Script/Squad.SQWorldSettings|GetMapTextureCornerZero _assqworld_settings)))) (.Y (Math|Vector|BreakVector (Transformation|GetActorLocation (Variables|/Script/Squad.SQWorldSettings|GetMapTextureCornerOne _assqworld_settings)))))))))
  (bind _output_get (LocalVariables|SetForbiddenCaptureZones (Variables|Default|GetMainBases)))
  (Utilities|IsValid _currentflag
    (:Is%20Valid
      (Utilities|Array|Add _output_get _currentflag))
    (:Is%20Not%20Valid
      _))
  (for _array_element (LocalVariables|GetForbiddenCaptureZones)
    (Utilities|Array|Add (LocalVariables|GetLocalInstructions) (Utilities|Struct|MakeMSPOverlayDrawingInstruction false (* 2.0 (Components|Sphere|GetScaledSphereRadius (Variables|/Game/Blueprints/Placeable/CaptureZones/BP_PSCaptureZoneNew.BP_PSCaptureZoneNew_C|GetSphere _array_element)) (LocalVariables|GetWorldScale)) (Utilities|WorldtoTextureSpaceLocation (LocalVariables|GetCornerZeroLoc) (LocalVariables|GetCornerOneLoc) (Transformation|GetActorLocation _array_element)) 0.0)))
  (return (LocalVariables|GetLocalInstructions)))

(fn DebugShowAllFlags
  (bind _outactors (Actor|GetAllActorsOfClass "/Game/Blueprints/Placeable/CaptureZones/BP_PSCaptureZoneNew.BP_PSCaptureZoneNew_C"))
  (Variables|Default|SetMainBases _outactors))