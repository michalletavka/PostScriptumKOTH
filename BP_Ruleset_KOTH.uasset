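; King of the Hill ruleset that activates one capture zone at a time, bleeding the non-holding team's tickets every second.
; On authority, it hides and shuffles flags, favouring a first one roughly equidistant from main bases.
; A one-second timer runs breaks and owned-flag countdowns via the KOTH Lattice, disables FOB spawns and destroys rallies inside the active zone.
; When the last flag expires, the team with more tickets wins.
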(event Custom|FlagExpired
  (params (CaptureZoneComponent :type BP%20PS%20Capture%20Zone%20Component%20Object%20Reference) (team :type ESQTeam%20Enum :default "Team_Neutral"))
  (bind _availableflags (Variables|Default|GetAvailableFlags))
  (bind _lattice (Variables|Default|GetLattice))
  (Networking|SwitchHasAuthority
    (:Authority
      (CallFunction|SetTeamsCanCapture CaptureZoneComponent false)
      (Variables|Default|SetCurrentFlagOwner "Team_Neutral")
      (Variables|/KOTH/GameMode/BP_PS_KOTH_Lattice.BP_PS_KOTH_Lattice_C|SetBreakRemainingTime _lattice (Variables|/KOTH/GameMode/BP_PS_KOTH_Lattice.BP_PS_KOTH_Lattice_C|GetBreakDuration _lattice))
      (if (>= (Utilities|Array|FindItem _availableflags (Variables|Default|GetCurrentFlag)) (- (Utilities|Array|Length _availableflags) 1))
        (CallFunction|AllFlagsCaptured)))))

(event Custom|AllFlagsCaptured
  (bind _winningteam (CallFunction|GetWinner))
  (bind _asbp_ps_game_mode (Utilities|Casting|CastToBP_PS_GameMode (Game|GetGameMode)))
  (Default|ForceEndMatch _asbp_ps_game_mode (Utilities|Select :Index _winningteam :Team_Neutral 0 :Team_One 1 :Team_Two 2)))

(event Custom|FlagOwnerChanged
  (params (CaptureZoneComponent :type BP%20PS%20Capture%20Zone%20Component%20Object%20Reference) (team :type ESQTeam%20Enum :default "Team_Neutral"))
  (Variables|Default|SetCurrentFlagOwner team))

(event Custom|BreakExpired
  (bind _lattice (Variables|Default|GetLattice))
  (Networking|SwitchHasAuthority
    (:Authority
      (bind _spawnedflag (CallFunction|SpawnNextFlag))
      (Default|CallOnBreakExpired)
      (Utilities|IsValid (Variables|/Game/Blueprints/Placeable/CaptureZones/BP_CaptureZone.BP_CaptureZone_C|GetBP_PSCaptureZoneComponent _spawnedflag)
        (:Is%20Valid
          (EventDispatchers|BindEventtoOnCaptureChange (Variables|/Game/Blueprints/Placeable/CaptureZones/BP_CaptureZone.BP_CaptureZone_C|GetBP_PSCaptureZoneComponent _spawnedflag) (delegate Custom|FlagOwnerChanged))
          (bind _output_get (Variables|Default|SetCurrentFlag _spawnedflag))
          (Variables|/KOTH/GameMode/BP_PS_KOTH_Lattice.BP_PS_KOTH_Lattice_C|SetCurrentFlag _lattice _output_get)
          (Variables|Default|SetCurrentFlagRemainingTime (Variables|/KOTH/GameMode/BP_PS_KOTH_Lattice.BP_PS_KOTH_Lattice_C|GetFlagDuration _lattice)))))))

(event Custom|BleedTickets
  (bind _currentflagowner (Variables|Default|GetCurrentFlagOwner))
  (bind _asbp_ps_game_mode (Utilities|Casting|CastToBP_PS_GameMode (Game|GetGameMode)))
  (if (not (Class|GameMode|HasMatchEnded _asbp_ps_game_mode))
    (if (Utilities|Enum|NotEqual(Enum) _currentflagowner "Team_Neutral")
      (bind _oppositeteam (CallFunction|GetOppositeTeam _currentflagowner))
      (Variables|/Script/Squad.SQTeamState|SetTickets (Utilities|Array|Get(acopy) (Variables|/Script/Squad.SQGameState|GetTeamStates (CallFunction|GetSquadGameState)) (Utilities|Select :Index _oppositeteam :Team_Neutral 0 :Team_One 0 :Team_Two 1)) (- (Variables|/Script/Squad.SQTeamState|GetTickets (Utilities|Array|Get(acopy) (Variables|/Script/Squad.SQGameState|GetTeamStates (CallFunction|GetSquadGameState)) (Utilities|Select :Index _oppositeteam :Team_Neutral 0 :Team_One 0 :Team_Two 1))) (Math|Float|Truncate (Variables|/KOTH/GameMode/BP_PS_KOTH_Lattice.BP_PS_KOTH_Lattice_C|GetTicketBleed (Variables|Default|GetLattice))))))))

(event EventBeginPlay
  (bind _lattice (Variables|Default|GetLattice))
  (Networking|SwitchHasAuthority
    (:Authority
      (|CallParentFunction)
      (CallFunction|InitFlags)
      (Utilities|Time|SetTimerbyEvent (delegate Custom|BleedTickets) 1.0 true)
      (Utilities|Time|SetTimerbyFunctionName 0 "OneSecondUpdater" 1.0 true)
      (Variables|/KOTH/GameMode/BP_PS_KOTH_Lattice.BP_PS_KOTH_Lattice_C|SetBreakRemainingTime _lattice (Variables|/KOTH/GameMode/BP_PS_KOTH_Lattice.BP_PS_KOTH_Lattice_C|GetStartGameBreakDuration _lattice)))))

(event Collision|EventActorBeginOverlap
  (params (OtherActor :type Actor%20Object%20Reference)))

(event EventRegisterActor
  (params (actor :type Actor%20Object%20Reference)))

(fn ConstructionScript
  (bind _asbp_ps_game_mode_koth (Utilities|Casting|CastToBP_PS_GameMode_KOTH (Game|GetGameMode)))
  (Default|OnRulesetRegistered _asbp_ps_game_mode_koth self)
  (bind _outactors (Actor|GetAllActorsOfClass "/KOTH/GameMode/BP_PS_KOTH_Lattice.BP_PS_KOTH_Lattice_C"))
  (bind _output_get (Variables|Default|SetLattice (Utilities|Array|Get(acopy) _outactors)))
  (bind _outactors_2 (Actor|GetAllActorsOfClass "/Game/Blueprints/Placeable/CaptureZones/BP_PSCaptureZoneMainNew.BP_PSCaptureZoneMainNew_C"))
  (Variables|/KOTH/GameMode/BP_PS_KOTH_Lattice.BP_PS_KOTH_Lattice_C|SetMainBases _output_get _outactors_2))

(fn InitFlags
  (bind _outactors (Actor|GetAllActorsOfClass "/Game/Blueprints/Placeable/CaptureZones/BP_PSCaptureZoneNew.BP_PSCaptureZoneNew_C"))
  (for _array_element _outactors
    (if (not (Variables|/Game/Blueprints/Placeable/CaptureZones/BP_PSCaptureZoneNew.BP_PSCaptureZoneNew_C|GetbIsMain _array_element))
      ;[1 1 1] Scale down the sphere to allow rallies to be put into inactive objectives
      (Transformation|SetActorScale3D _array_element "0, 0, 0")
      (Utilities|Array|Add (Variables|Default|GetAvailableFlags) _array_element)
      (Utilities|Array|Shuffle (Variables|Default|GetAvailableFlags))
      (Variables|/Script/Squad.SQMapItemComponent|SetbIsVisible (Variables|/Game/Blueprints/Placeable/CaptureZones/BP_PSCaptureZoneNew.BP_PSCaptureZoneNew_C|GetSQMapIcon _array_element) false)
      (CallFunction|SetTeamsCanCapture (Variables|/Game/Blueprints/Placeable/CaptureZones/BP_CaptureZone.BP_CaptureZone_C|GetBP_PSCaptureZoneComponent _array_element) false)
      (Variables|/Script/Squad.SQCaptureZoneComponent|SetTimeToCap (Variables|/Game/Blueprints/Placeable/CaptureZones/BP_CaptureZone.BP_CaptureZone_C|GetBP_PSCaptureZoneComponent _array_element) 1.0)
      (Variables|/Script/Squad.SQCaptureZoneComponent|SetPlayerAdvantageToCapture (Variables|/Game/Blueprints/Placeable/CaptureZones/BP_CaptureZone.BP_CaptureZone_C|GetBP_PSCaptureZoneComponent _array_element) 1)
      (Variables|/Script/Squad.SQCaptureZoneComponent|SetPlayersNeededWhenUncaptured (Variables|/Game/Blueprints/Placeable/CaptureZones/BP_CaptureZone.BP_CaptureZone_C|GetBP_PSCaptureZoneComponent _array_element) 1)
      (Variables|/Game/PostScriptum/Blueprints/BP_PSCaptureZoneComponent.BP_PSCaptureZoneComponent_C|SetbVisibleForTeam (Variables|/Game/Blueprints/Placeable/CaptureZones/BP_CaptureZone.BP_CaptureZone_C|GetBP_PSCaptureZoneComponent _array_element) (Utilities|Array|MakeArray false false false))))
  (CallFunction|ChoseBestFirstFlag))

(fn SpawnNextFlag
  (bind _flag (CallFunction|GetNextFlag))
  (Variables|/Script/Squad.SQMapItemComponent|SetbIsVisible (Variables|/Game/Blueprints/Placeable/CaptureZones/BP_PSCaptureZoneNew.BP_PSCaptureZoneNew_C|GetSQMapIcon _flag) true)
  (CallFunction|SetTeamsCanCapture (Variables|/Game/Blueprints/Placeable/CaptureZones/BP_CaptureZone.BP_CaptureZone_C|GetBP_PSCaptureZoneComponent _flag) true)
  (Variables|/Game/PostScriptum/Blueprints/BP_PSCaptureZoneComponent.BP_PSCaptureZoneComponent_C|SetbVisibleForTeam (Variables|/Game/Blueprints/Placeable/CaptureZones/BP_CaptureZone.BP_CaptureZone_C|GetBP_PSCaptureZoneComponent _flag) (Utilities|Array|MakeArray true true true))
  (Transformation|SetActorScale3D _flag "1.000000,1.000000,1.000000")
  (return _flag))

(fn SetTeamsCanCapture
  (params (Flag :type BP%20PS%20Capture%20Zone%20Component%20Object%20Reference%20%28by%20ref%29) (CanCapture :type Boolean))
  (Class|SQCaptureZoneComponent|SetTeamCanCapture Flag 0 CanCapture)
  (Class|SQCaptureZoneComponent|SetTeamCanCapture Flag 1 CanCapture)
  (Class|SQCaptureZoneComponent|SetTeamCanCapture Flag 2 CanCapture)
  (if CanCapture
    (Class|SQCaptureZoneComponent|UnlockCaptureZone Flag)
    (else
      (Class|SQCaptureZoneComponent|LockCaptureZone Flag))))

(fn GetNextFlag
  (bind _array_element (Utilities|Array|ForEachLoopwithBreak (Variables|Default|GetAvailableFlags))
    (:LoopBody
      (if (not (Variables|/Script/Squad.SQMapItemComponent|GetbIsVisible (Variables|/Game/Blueprints/Placeable/CaptureZones/BP_PSCaptureZoneNew.BP_PSCaptureZoneNew_C|GetSQMapIcon _array_element)))
        (return _array_element)))))

(fn GetOppositeTeam
  (params (ThisTeam :type ESQTeam%20Enum :default "Team_Neutral"))
  (if (Utilities|Enum|Equal(Enum) ThisTeam "Team_Neutral")
    (return "Team_Neutral")
    (elif (Utilities|Enum|Equal(Enum) ThisTeam "Team_Two")
      (return "Team_One")
      (else
        (return "Team_Two")))))

(fn GetWinner
  (bind _return_value (CallFunction|GetSquadGameState))
  (bind _teamstates (Variables|/Script/Squad.SQGameState|GetTeamStates _return_value))
  (bind _output (Utilities|Array|Get(acopy) _teamstates))
  (bind _output_2 (Utilities|Array|Get(acopy) _teamstates 1))
  (bind _tickets (Variables|/Script/Squad.SQTeamState|GetTickets _output))
  (bind _tickets_2 (Variables|/Script/Squad.SQTeamState|GetTickets _output_2))
  (if (== _tickets _tickets_2)
    (return "Team_Neutral")
    (elif (> _tickets _tickets_2)
      (return "Team_One")
      (else
        (return "Team_Two")))))

(fn UpdateActiveTimeLeft
  (bind _currentflag (Variables|Default|GetCurrentFlag))
  (bind _bp_pscapturezonecomponent (Variables|/Game/Blueprints/Placeable/CaptureZones/BP_CaptureZone.BP_CaptureZone_C|GetBP_PSCaptureZoneComponent _currentflag))
  (Utilities|IsValid _currentflag
    (:Is%20Valid
      (if (Utilities|Enum|NotEqual(Enum) (Variables|Default|GetCurrentFlagOwner) "Team_Neutral")
        (bind _output_get (Variables|Default|SetCurrentFlagRemainingTime (- (Variables|Default|GetCurrentFlagRemainingTime) 1.0))))
      (Variables|/KOTH/GameMode/BP_PS_KOTH_Lattice.BP_PS_KOTH_Lattice_C|SetActiveFlagRemainingTime (Variables|Default|GetLattice) _output_get)
      (if (<= _output_get 0.0)
        (Variables|Default|SetCurrentFlagRemainingTime 1e+10)
        (Class|SQCaptureZoneComponent|FullyCap _bp_pscapturezonecomponent (Variables|/Script/Squad.SQCaptureZoneComponent|GetLastOwningTeam _bp_pscapturezonecomponent))
        (CallFunction|FlagExpired _bp_pscapturezonecomponent "Team_Neutral")))))

(fn IsPlayerinFlag
  (params (Flag :type BP%20PS%20Capture%20Zone%20New%20Object%20Reference) (Panel :type Canvas%20Panel%20Object%20Reference))
  (bind _returnvalue (Game|GetPlayerController 0))
  (Utilities|IsValid Panel
    (:Is%20Valid
      (Utilities|IsValid _returnvalue
        (:Is%20Valid
          (Utilities|IsValid Flag
            (:Is%20Valid
              (return (> (Math|Float|Square (Components|Sphere|GetScaledSphereRadius (Variables|/Game/Blueprints/Placeable/CaptureZones/BP_PSCaptureZoneNew.BP_PSCaptureZoneNew_C|GetSphere Flag))) (Math|Vector|VectorLengthSquared (- (Transformation|GetActorLocation Flag) (Transformation|GetActorLocation _returnvalue))))))))
        (:Is%20Not%20Valid
          _)))
    (:Is%20Not%20Valid
      _))
  (return false))

(fn InitFlagsClient
  (bind _outactors (Actor|GetAllActorsOfClass "/Game/Blueprints/Placeable/CaptureZones/BP_PSCaptureZoneNew.BP_PSCaptureZoneNew_C"))
  (for _array_element _outactors
    (if (not (Variables|/Game/Blueprints/Placeable/CaptureZones/BP_PSCaptureZoneNew.BP_PSCaptureZoneNew_C|GetbIsMain _array_element))
      (Variables|/Script/Squad.SQMapItemComponent|SetbIsVisible (Variables|/Game/Blueprints/Placeable/CaptureZones/BP_PSCaptureZoneNew.BP_PSCaptureZoneNew_C|GetSQMapIcon _array_element) false)
      (CallFunction|SetTeamsCanCapture (Variables|/Game/Blueprints/Placeable/CaptureZones/BP_CaptureZone.BP_CaptureZone_C|GetBP_PSCaptureZoneComponent _array_element) false))))

(fn UpdateBreakTimeLeft
  (if (> (Variables|/KOTH/GameMode/BP_PS_KOTH_Lattice.BP_PS_KOTH_Lattice_C|GetBreakRemainingTime (Variables|Default|GetLattice)) 0.0)
    (Variables|/KOTH/GameMode/BP_PS_KOTH_Lattice.BP_PS_KOTH_Lattice_C|SetBreakRemainingTime (Variables|Default|GetLattice) (- (Variables|/KOTH/GameMode/BP_PS_KOTH_Lattice.BP_PS_KOTH_Lattice_C|GetBreakRemainingTime (Variables|Default|GetLattice)) 1.0))
    (Variables|Default|SetIsBreakActive true)
    (elif (Variables|Default|GetIsBreakActive)
      (Variables|Default|SetIsBreakActive false)
      (CallFunction|BreakExpired))))

(fn ChoseBestFirstFlag
  (bind _candidateflags (LocalVariables|GetCandidateFlags))
  (bind _availableflags (Variables|Default|GetAvailableFlags))
  (bind _lattice (Variables|Default|GetLattice))
  (bind _mainbases (Variables|/KOTH/GameMode/BP_PS_KOTH_Lattice.BP_PS_KOTH_Lattice_C|GetMainBases _lattice))
  (if (<= (Utilities|Array|Length (Variables|Default|GetAvailableFlags)) (LocalVariables|GetMinAmountOfCandidates))
    (return)
    (else
      (LocalVariables|SetMainBaseA (Transformation|GetActorLocation (Utilities|Array|Get(acopy) _mainbases)))
      (LocalVariables|SetMainBaseB (Transformation|GetActorLocation (Utilities|Array|Get(acopy) _mainbases 1)))
      (while (< (Utilities|Array|Length (LocalVariables|GetCandidateFlags)) (LocalVariables|GetMinAmountOfCandidates))
        (for _array_element (Variables|Default|GetAvailableFlags)
          (if (not (Utilities|Array|ContainsItem (LocalVariables|GetCandidateFlags) _array_element))
            (if (<= (Math|Integer|Absolute(Integer) (- (Math|Float|Truncate (Math|Float|Sqrt (Math|Float|Absolute(Float) (Math|Vector|VectorLengthSquared (- (LocalVariables|GetMainBaseA) (Transformation|GetActorLocation _array_element)))))) (Math|Float|Truncate (Math|Float|Sqrt (Math|Float|Absolute(Float) (Math|Vector|VectorLengthSquared (- (Transformation|GetActorLocation _array_element) (LocalVariables|GetMainBaseB)))))))) (LocalVariables|GetDistanceThreshold))
              (Utilities|Array|Add (LocalVariables|GetCandidateFlags) _array_element))))
        (LocalVariables|SetDistanceThreshold (+ (LocalVariables|GetDistanceThreshold) (LocalVariables|GetDistanceThresholdStep))))
      (bind _output_get (LocalVariables|SetBestCandidate (Utilities|Array|Get(acopy) _candidateflags (Math|Random|RandomIntegerinRange 0 (Utilities|Array|Length _candidateflags)))))
      (Utilities|Array|RemoveItem _availableflags _output_get)
      (Utilities|Array|Insert _availableflags _output_get))))

(fn DebugShowAllFlags
  (bind _outactors (Actor|GetAllActorsOfClass "/Game/Blueprints/Placeable/CaptureZones/BP_PSCaptureZoneNew.BP_PSCaptureZoneNew_C"))
  (for _array_element _outactors
    (if (not (Variables|/Game/Blueprints/Placeable/CaptureZones/BP_PSCaptureZoneNew.BP_PSCaptureZoneNew_C|GetbIsMain _array_element))
      (Utilities|Array|Add (Variables|Default|GetAvailableFlags) _array_element)
      (Utilities|Array|Shuffle (Variables|Default|GetAvailableFlags))
      (Variables|/Script/Squad.SQMapItemComponent|SetbIsVisible (Variables|/Game/Blueprints/Placeable/CaptureZones/BP_PSCaptureZoneNew.BP_PSCaptureZoneNew_C|GetSQMapIcon _array_element) true)
      (CallFunction|SetTeamsCanCapture (Variables|/Game/Blueprints/Placeable/CaptureZones/BP_CaptureZone.BP_CaptureZone_C|GetBP_PSCaptureZoneComponent _array_element) true)
      (Variables|/Game/PostScriptum/Blueprints/BP_PSCaptureZoneComponent.BP_PSCaptureZoneComponent_C|SetbVisibleForTeam (Variables|/Game/Blueprints/Placeable/CaptureZones/BP_CaptureZone.BP_CaptureZone_C|GetBP_PSCaptureZoneComponent _array_element) (Utilities|Array|MakeArray true true true))
      (Default|DebugShowAllFlags (Variables|Default|GetLattice)))))

(fn UpdateFobsinCap
  (bind _outactors (Actor|GetAllActorsOfClass "/Game/PostScriptum/Gameplay/Deployables/BP_PS_BaseFobCreator.BP_PS_BaseFobCreator_C"))
  (for _array_element _outactors
    (bind _incurrentflag (CallFunction|IsinCurrentFlag (Transformation|GetActorLocation _array_element)))
    (if _incurrentflag
      (if (and (not (Class|SQDeployable|IsGhost _array_element)) (Variables|/Script/Squad.SQForwardBase|GetbIsSpawningEnabled _array_element))
        (Default|DestroySpawn _array_element)
        ;[1 1 1] workaround for internal BP_PS_BaseFobCreator logic that would CreateSpawns every 2 seconds
        (Variables|/Game/PostScriptum/Gameplay/Deployables/BP_PS_BaseFobCreator.BP_PS_BaseFobCreator_C|SetIsSpawnEnabled _array_element true))
      (elif (not (Variables|/Script/Squad.SQForwardBase|GetbIsSpawningEnabled _array_element))
        (Default|CreateSpawn _array_element)))))

(fn OneSecondUpdater
  (Utilities|FlowControl|Sequence
    (:then_0
      (CallFunction|UpdateActiveTimeLeft))
    (:then_1
      (CallFunction|UpdateBreakTimeLeft))
    (:then_2
      (CallFunction|UpdateFobsinCap))
    (:then_3
      (CallFunction|UpdateRallysinCap))))

(fn IsinCurrentFlag
  (params (Location :type Vector))
  (bind _currentflag (Variables|Default|GetCurrentFlag))
  (Utilities|IsValid _currentflag
    (:Is%20Valid
      (return (> (Math|Float|Square (Components|Sphere|GetScaledSphereRadius (Variables|/Game/Blueprints/Placeable/CaptureZones/BP_PSCaptureZoneNew.BP_PSCaptureZoneNew_C|GetSphere _currentflag))) (Math|Vector|VectorLengthSquared (- Location (Transformation|GetActorLocation _currentflag))))))
    (:Is%20Not%20Valid
      (return false))))

(fn UpdateRallysinCap
  (bind _outactors (Actor|GetAllActorsOfClass "/Game/PostScriptum/Gameplay/Section/BP_RadioRecallSpawn.BP_RadioRecallSpawn_C"))
  (for _array_element _outactors
    (bind _incurrentflag (CallFunction|IsinCurrentFlag (Transformation|GetActorLocation _array_element)))
    (if _incurrentflag
      (if (Variables|/Script/Squad.SQGameSpawn|GetbSpawningEnabled _array_element)
        (Actor|DestroyActor _array_element)))))